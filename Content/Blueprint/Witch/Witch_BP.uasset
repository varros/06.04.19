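; Witch_BP is a player witch Blueprint that handles damage, death and respawning.
; Capsule hits from Enemy_BP actors reduce HealthNew, reloading Level1 when it runs out and otherwise printing a damage message.
; The Respawn input destroys the actor, spawns a new Witch at SpawnLocation and has player controller 0 possess it.
; The X key triggers a spawn at the world origin with no class shown.
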(event OnComponentHit(CapsuleComponent)
  (params (HitComponent :type Primitive%20Component%20Object%20Reference) (OtherActor :type Actor%20Object%20Reference) (OtherComp :type Primitive%20Component%20Object%20Reference) (NormalImpulse :type Vector :default "0, 0, 0") (Hit :type Hit%20Result%20Structure%20%28by%20ref%29))
  ;[1 1 1] Enemy hurts and kills player
  (Utilities|Casting|CastToEnemy_BP OtherActor)
  (Variables|Default|SetHealth_New (- (Variables|Default|GetHealth_New) 10))
  (if (<= (Variables|Default|GetHealth_New) 0)
    (Game|OpenLevel(byName) "Level1")
    (Development|PrintString "You died")
    (else
      (Development|PrintString "Damage"))))

(event Input|ActionEvents|InputActionRespawn
  (params (Key :type Key%20Structure))
  ;[1 1 1] Call Respawn
  (:Released
    (Actor|DestroyActor)
    (CallFunction|RespawnPlayer (Variables|Default|GetSpawn%20Location))))

(event Input|KeyboardEvents|X
  (params (Key :type Key%20Structure))
  (:Pressed
    (Game|SpawnActorfromClass "/Game/Blueprint/Witch/Projectile_BP.Projectile_BP_C" (Math|Transform|MakeTransform "0, 0, 0") "Undefined" 0 0)))

(fn ConstructionScript)

(fn RespawnPlayer
  (params (SpawnTransform :type Transform))
  ;[1 1 1] Respawn Player
  (bind _returnvalue (Game|SpawnActorfromClass "/Script/Witch_Hunt.Witch" SpawnTransform "Undefined" 0 0))
  (Pawn|Possess (Game|GetPlayerController 0) _returnvalue))